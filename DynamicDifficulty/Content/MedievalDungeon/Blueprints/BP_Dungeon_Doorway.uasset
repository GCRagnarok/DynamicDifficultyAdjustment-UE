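; Dungeon doorway actor with a large double door that swings open when its OpenDoor event fires.
; OpenDoor prints a debug string, then plays a Timeline that lerps the right leaf's relative rotation through a quarter turn and mirrors it on the left.
; Unconnected blood-lock logic would count dead undead enemies against the array length, but it never runs and does not trigger the door.
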(event `self.ReceiveBeginPlay`)

(event `self.ReceiveTick`
  (params (DeltaSeconds :type "Float (single-precision)")))

(event `OpenDoor`
  (`KismetSystemLibrary.PrintString` "Hello")
  (bind (_direction _newtrack_0) (`Timeline|Timeline` :!via `PlayFromStart`)
    (:`Update`
      (bind _returnvalue (`KismetMathLibrary.RLerp` (struct) (struct :`Yaw` -90.0) _newtrack_0))
      (`SceneComponent.K2_SetRelativeRotation` (`self.SM_DoorWay_Large_Door_Right`) _returnvalue false false)
      (`SceneComponent.K2_SetRelativeRotation` (`self.SM_DoorWay_Large_Door_Left`) (* _returnvalue -1.0) false false))))

(fn `UserConstructionScript`)