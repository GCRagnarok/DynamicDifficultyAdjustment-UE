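; BP_ky_thunderBall is a thunder ball effect actor that bursts on contact with players or walls.
; Its Box overlap ignores actors whose first tag is ky_shot, then accepts Player-tagged actors, except through LockOn-tagged components, or Wall-tagged actors.
; A valid hit spawns the HitFx emitter at the box location and destroys the actor.
; The graph applies no damage or movement.
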(event `self.ReceiveActorBeginOverlap`
  (params (OtherActor :type "Actor Object Reference")))

(event `self.Box.OnComponentBeginOverlap`
  (params (OverlappedComponent :type "PrimitiveComponent Object Reference") (OtherActor :type "Actor Object Reference") (OtherComp :type "PrimitiveComponent Object Reference") (OtherBodyIndex :type Integer) (bFromSweep :type Boolean) (SweepResult :type "HitResult Structure (by ref)"))
  ;[1 1 1] spawn collison fx
  (if (`KismetSystemLibrary.IsValid` OtherActor)
    (if (!= (`|GetArrayItem` (`Actor.Tags` OtherActor)) "ky_shot")
      (if (or (and (`self.ActorHasTag` OtherActor "Player") (not (`ActorComponent.ComponentHasTag` OtherComp "LockOn"))) (`self.ActorHasTag` OtherActor "Wall"))
        (`GameplayStatics.SpawnEmitterAtLocation` (`self.hitFx`) (`SceneComponent.K2_GetComponentLocation` (`self.Box`)))
        ;[1 1 1] fx destroy
        (`self.K2_DestroyActor`)))))

(fn `UserConstructionScript`
  (`parent.UserConstructionScript`))